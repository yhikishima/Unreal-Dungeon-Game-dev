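; BP_ItemBox is an item box that opens on being hit and grants the player a weapon.
; A DoOnce on Hit precedes the BP_Player cast, so only the first hit by any actor is processed.
; For a player, it shows WBP_ItemGet and swaps to the opened mesh.
; The widget's remove event is bound to RemoveItemGet, which calls GetWeapon on BP_GameInstance and removes the widget.
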(event Custom|RemoveItemGet
  (bind _asbp_game_instance (Utilities|Casting|CastToBP_GameInstance (Game|GetGameInstance)))
  (Default|GetWeapon _asbp_game_instance)
  (Widget|RemovefromParent (stale Collision|EventHit _returnvalue)))

(event EventBeginPlay)

(event Collision|EventActorBeginOverlap
  (params (OtherActor :type Actor%20Object%20Reference)))

(event EventTick
  (params (DeltaSeconds :type Float%20%28single-precision%29)))

(event Collision|EventHit
  (params (MyComp :type Primitive%20Component%20Object%20Reference) (Other :type Actor%20Object%20Reference) (OtherComp :type Primitive%20Component%20Object%20Reference) (bSelfMoved :type Boolean) (HitLocation :type Vector :default "0, 0, 0") (HitNormal :type Vector :default "0, 0, 0") (NormalImpulse :type Vector :default "0, 0, 0") (Hit :type Hit%20Result%20Structure%20%28by%20ref%29))
  (Utilities|FlowControl|DoOnce false
    (:Completed
      (Utilities|Casting|CastToBP_Player Other)
      (bind _returnvalue (UserInterface|CreateWidget "/Game/Ui/WBP_ItemGet.WBP_ItemGet_C"))
      (UserInterface|Viewport|AddtoViewport _returnvalue 0)
      (EventDispatchers|BindEventtoRemoveSelf _returnvalue (delegate Custom|RemoveItemGet))
      (Components|StaticMesh|SetStaticMesh (Variables|Debug|GetStaticMeshComponent) "/Game/ItemboxPackII/Meshes/SM_ItemboxII10Opened.SM_ItemboxII10Opened"))))

(fn ConstructionScript)