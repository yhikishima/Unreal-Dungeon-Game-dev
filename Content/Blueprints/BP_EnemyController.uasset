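; BP_EnemyController is an enemy Blueprint that takes damage from the player and is removed when defeated.
; Its Attack graph handles Hit events, casts the other actor to BP_Player and subtracts one EnemyHp per hit, without checking which component struck.
; The actor is destroyed only once EnemyHp drops below zero; otherwise it prints the remaining HP.
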(event EventBeginPlay)

(event Collision|EventActorBeginOverlap
  (params (OtherActor :type Actor%20Object%20Reference)))

(event EventTick
  (params (DeltaSeconds :type Float%20%28single-precision%29)))

(event Collision|EventHit
  (params (MyComp :type Primitive%20Component%20Object%20Reference) (Other :type Actor%20Object%20Reference) (OtherComp :type Primitive%20Component%20Object%20Reference) (bSelfMoved :type Boolean) (HitLocation :type Vector :default "0, 0, 0") (HitNormal :type Vector :default "0, 0, 0") (NormalImpulse :type Vector :default "0, 0, 0") (Hit :type Hit%20Result%20Structure%20%28by%20ref%29))
  ;[1 1 1] ダメージくらう
  (bind _asbp_player (Utilities|Casting|CastToBP_Player Other))
  (bind _output_get (Variables|Default|SetEnemyHp (- (Variables|Default|GetEnemyHp) 1)))
  ;[1 1 1] 討伐
  (if (> 0 _output_get)
    (Actor|DestroyActor)
    (else
      (Development|PrintString (Utilities|String|ToString(Integer) (Variables|Default|GetEnemyHp))))))

(fn ConstructionScript)