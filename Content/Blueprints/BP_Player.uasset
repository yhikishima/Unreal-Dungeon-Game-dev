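; Player Blueprint that handles damage from enemies, game over and showing a sword.
; Capsule hits from BP_EnemyController subtract 1 HP, then either add WBP_GameOver to the viewport once HP drops below zero or briefly raise IsHitting for damage display.
; SetSword makes RightSword visible, while hit and overlap events on RightSword and SwordCollision only print debug strings.
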(event OnComponentHit(CapsuleComponent)
  (params (HitComponent :type Primitive%20Component%20Object%20Reference) (OtherActor :type Actor%20Object%20Reference) (OtherComp :type Primitive%20Component%20Object%20Reference) (NormalImpulse :type Vector :default "0, 0, 0") (Hit :type Hit%20Result%20Structure%20%28by%20ref%29))
  (Utilities|Casting|CastToBP_EnemyController OtherActor)
  ;[1 1 1] ダメージくらう
  (Variables|Default|SetHP (- (Variables|Default|GetHP) 1))
  (if (< (Variables|Default|GetHP) 0)
    ;[1 1 1] ゲームオーバー
    (bind _returnvalue (UserInterface|CreateWidget "/Game/Ui/WBP_GameOver.WBP_GameOver_C"))
    (UserInterface|Viewport|AddtoViewport _returnvalue 0)
    (else
      ;[1 1 1] ダメージ表示
      (if (not (Variables|Default|GetIsHitting))
        (Variables|Default|SetIsHitting true)
        (Utilities|FlowControl|Delay 0.2)
        (Variables|Default|SetIsHitting false)))))

(event OnComponentHit(SwordCollision)
  (params (HitComponent :type Primitive%20Component%20Object%20Reference) (OtherActor :type Actor%20Object%20Reference) (OtherComp :type Primitive%20Component%20Object%20Reference) (NormalImpulse :type Vector :default "0, 0, 0") (Hit :type Hit%20Result%20Structure%20%28by%20ref%29))
  (Development|PrintString "Hello"))

(event OnComponentHit(RightSword)
  (params (HitComponent :type Primitive%20Component%20Object%20Reference) (OtherActor :type Actor%20Object%20Reference) (OtherComp :type Primitive%20Component%20Object%20Reference) (NormalImpulse :type Vector :default "0, 0, 0") (Hit :type Hit%20Result%20Structure%20%28by%20ref%29))
  (Development|PrintString "Hello"))

(event OnComponentBeginOverlap(RightSword)
  (params (OverlappedComponent :type Primitive%20Component%20Object%20Reference) (OtherActor :type Actor%20Object%20Reference) (OtherComp :type Primitive%20Component%20Object%20Reference) (OtherBodyIndex :type Integer) (bFromSweep :type Boolean) (SweepResult :type Hit%20Result%20Structure%20%28by%20ref%29))
  (Development|PrintString "Player Hit"))

(event OnComponentBeginOverlap(SwordCollision)
  (params (OverlappedComponent :type Primitive%20Component%20Object%20Reference) (OtherActor :type Actor%20Object%20Reference) (OtherComp :type Primitive%20Component%20Object%20Reference) (OtherBodyIndex :type Integer) (bFromSweep :type Boolean) (SweepResult :type Hit%20Result%20Structure%20%28by%20ref%29))
  (Development|PrintString (Utilities|GetDisplayName OtherActor)))

(event Custom|SetSword
  (Rendering|SetVisibility (Variables|Default|GetRightSword) true false))

(event EventBeginPlay)

(event Collision|EventActorBeginOverlap
  (params (OtherActor :type Actor%20Object%20Reference)))

(event EventTick
  (params (DeltaSeconds :type Float%20%28single-precision%29)))

(fn ConstructionScript)