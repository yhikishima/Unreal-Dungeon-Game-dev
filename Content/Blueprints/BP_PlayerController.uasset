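; BP_PlayerController is the player controller that drives BP_Player from input and shows the mouse cursor.
; MoveForward and MoveRight add movement along fixed world axes and snap the mesh yaw to four cardinal directions at full axis values.
; On BeginPlay it binds HasWeapon to BP_GameInstance's weapon-completion event, which calls SetSword on the player.
; The Attack input only toggles an Attacked flag on press and release.
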(event EventTick
  (params (DeltaSeconds :type Float%20%28single-precision%29)))

(event EventBeginPlay
  ;[1 1 1] 初期化
  (bind _asbp_player (Utilities|Casting|CastToBP_Player (Game|GetPlayerCharacter 0)))
  (bind _output_get (Variables|Default|SetBP_Player _asbp_player))
  (Variables|Default|SetbShowMouseCursor true)
  (CallFunction|SetWeapon))

(event Input|AxisEvents|InputAxisMoveForward
  (params (AxisValue :type Float%20%28single-precision%29))
  ;[1 1 1] 上下移動
  (Pawn|Input|AddMovementInput (stale EventBeginPlay _output_get) "-1.000000,0.000000,0.000000" AxisValue false)
  (if (>= AxisValue 1.0)
    (Transformation|SetRelativeRotation (Variables|/Script/Engine.Character|GetMesh (stale EventBeginPlay _output_get)) "0, 0, 0" false false)
    (elif (>= -1.0 AxisValue)
      (Transformation|SetRelativeRotation (Variables|/Script/Engine.Character|GetMesh (stale EventBeginPlay _output_get)) "0,180.000000, 0" false false))))

(event Input|AxisEvents|InputAxisMoveRight
  (params (AxisValue :type Float%20%28single-precision%29))
  ;[1 1 1] 左右移動
  (Pawn|Input|AddMovementInput (stale EventBeginPlay _output_get) "0.000000,-1.000000,0.000000" AxisValue false)
  (if (>= AxisValue 1.0)
    (Transformation|SetRelativeRotation (Variables|/Script/Engine.Character|GetMesh (stale EventBeginPlay _output_get)) "0,90.000000, 0" false false)
    (elif (>= -1.0 AxisValue)
      (Transformation|SetRelativeRotation (Variables|/Script/Engine.Character|GetMesh (stale EventBeginPlay _output_get)) "0,-90.000000, 0" false false))))

(event Custom|SetWeapon
  (bind _asbp_game_instance (Utilities|Casting|CastToBP_GameInstance (Game|GetGameInstance)))
  (EventDispatchers|BindEventtoCompleteWeapon _asbp_game_instance (delegate Custom|HasWeapon)))

(event Custom|HasWeapon
  (bind _asbp_player (Utilities|Casting|CastToBP_Player (Variables|Default|GetBP_Player)))
  (Default|SetSword _asbp_player))

(event Input|ActionEvents|InputActionAttack
  (params (Key :type Key%20Structure :default "None"))
  (:Pressed
    (Variables|Default|SetAttacked true))
  (:Released
    (Variables|Default|SetAttacked false)))

(fn ConstructionScript)