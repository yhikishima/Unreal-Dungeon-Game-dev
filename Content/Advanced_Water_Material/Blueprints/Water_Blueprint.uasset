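; Water surface actor that exposes the look of its Waterplane mesh as editable variables.
; Its construction script creates a dynamic material instance and pushes wave, color, refraction, shore, surge, tessellation, foam, rain and coral reef settings into it.
; Overall, foam, distortion, rain and reef scales are divided by the plane's summed X and Y world scale.
; Surge Speed is fed from SurgeHeight; the event graph is inactive.
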(event EventBeginPlay)

(event Collision|EventActorBeginOverlap
  (params (OtherActor :type Actor%20Object%20Reference)))

(event EventTick
  (params (DeltaSeconds :type Float%20%28single-precision%29)))

(fn ConstructionScript
  (bind _waterplane (Variables|Default|Getwaterplane))
  (bind _scale (Variables|Default|GetScale))
  (bind _waterplane_2 (Variables|Default|Getwaterplane))
  (bind _returnvalue (Transformation|GetWorldScale _waterplane))
  (bind _returnvalue_2 (Transformation|GetWorldScale _waterplane_2))
  (bind (_x _y) (Math|Vector|BreakVector _returnvalue))
  (bind (_x_2 _y_2) (Math|Vector|BreakVector _returnvalue_2))
  (bind _returnvalue_3 (+ _x _y))
  (bind _returnvalue_4 (+ _x_2 _y_2))
  (bind _returnvalue_5 (/ _scale _returnvalue_4))
  (bind _returnvalue_6 (Rendering|Material|CreateDynamicMaterialInstance _waterplane_2 0 "/Game/Advanced_Water_Material/Materials/Water_Material/Blueprint_Instance.Blueprint_Instance" "None" :!class /Script/Engine.PrimitiveComponent))
  (Rendering|Material|SetScalarParameterValue _returnvalue_6 "Overall Scale" _returnvalue_5 :!class /Script/Engine.MaterialInstanceDynamic)
  (Rendering|Material|SetScalarParameterValue _returnvalue_6 "Overall Normal Power" (Variables|Default|GetNormal%20Strength) :!class /Script/Engine.MaterialInstanceDynamic)
  (Rendering|Material|SetScalarParameterValue _returnvalue_6 "Metallic" (Variables|Default|GetMetallic) :!class /Script/Engine.MaterialInstanceDynamic)
  (Rendering|Material|SetScalarParameterValue _returnvalue_6 "Normal Fresnel Power" (Variables|Default|GetFresnel) :!class /Script/Engine.MaterialInstanceDynamic)
  (Rendering|Material|SetScalarParameterValue _returnvalue_6 "Ocean Normal Scale" (Variables|Default|GetOcean%20Waves%20Scale) :!class /Script/Engine.MaterialInstanceDynamic)
  (Rendering|Material|SetScalarParameterValue _returnvalue_6 "Wave Normal Scale" (Variables|Default|GetSmall%20Waves%20Scale) :!class /Script/Engine.MaterialInstanceDynamic)
  (Rendering|Material|SetScalarParameterValue _returnvalue_6 "Ocean Normal Speed" (Variables|Default|GetOcean%20Waves%20Speed) :!class /Script/Engine.MaterialInstanceDynamic)
  (Rendering|Material|SetScalarParameterValue _returnvalue_6 "Wave Normal Speed" (Variables|Default|GetSmall%20Waves%20Speed) :!class /Script/Engine.MaterialInstanceDynamic)
  (Rendering|Material|SetScalarParameterValue _returnvalue_6 "Ocean Normal Strength" (Variables|Default|GetOcean%20Normal%20Power) :!class /Script/Engine.MaterialInstanceDynamic)
  (Rendering|Material|SetScalarParameterValue _returnvalue_6 "Wave Normal Strength" (Variables|Default|GetWaves%20Normal%20Power) :!class /Script/Engine.MaterialInstanceDynamic)
  (Rendering|Material|SetScalarParameterValue _returnvalue_6 "Deep IQR" (Variables|Default|GetDeep%20Refraction) :!class /Script/Engine.MaterialInstanceDynamic)
  (Rendering|Material|SetScalarParameterValue _returnvalue_6 "Shallow IQR" (Variables|Default|GetShallow%20Refraction) :!class /Script/Engine.MaterialInstanceDynamic)
  (Rendering|Material|SetVectorParameterValue _returnvalue_6 "Color Deep" (Math|Conversions|ToLinearColor(Color) (Variables|Default|GetDeep%20Color)) :!class /Script/Engine.MaterialInstanceDynamic)
  (Rendering|Material|SetVectorParameterValue _returnvalue_6 "Color Shallow" (Math|Conversions|ToLinearColor(Color) (Variables|Default|GetShallow%20Color)) :!class /Script/Engine.MaterialInstanceDynamic)
  (Rendering|Material|SetScalarParameterValue _returnvalue_6 "Color Smooth" (Variables|Default|GetSmooth%20Color) :!class /Script/Engine.MaterialInstanceDynamic)
  (Rendering|Material|SetScalarParameterValue _returnvalue_6 "Color Spread" (Variables|Default|GetSpread%20Color) :!class /Script/Engine.MaterialInstanceDynamic)
  (Rendering|Material|SetScalarParameterValue _returnvalue_6 "Deep Opacity" (Variables|Default|GetDeep%20Opacity) :!class /Script/Engine.MaterialInstanceDynamic)
  (Rendering|Material|SetScalarParameterValue _returnvalue_6 "Shallow Opacity" (Variables|Default|GetShallow%20Opacity) :!class /Script/Engine.MaterialInstanceDynamic)
  (Rendering|Material|SetScalarParameterValue _returnvalue_6 "Water Height" (Variables|Default|GetWater%20Height) :!class /Script/Engine.MaterialInstanceDynamic)
  (Rendering|Material|SetScalarParameterValue _returnvalue_6 "Shore Depth" (Variables|Default|GetShore%20Depth) :!class /Script/Engine.MaterialInstanceDynamic)
  (Rendering|Material|SetScalarParameterValue _returnvalue_6 "Surge Divisor" (Variables|Default|GetSurge%20Divisor) :!class /Script/Engine.MaterialInstanceDynamic)
  (Rendering|Material|SetScalarParameterValue _returnvalue_6 "Surge Speed" (Variables|Default|GetSurge%20Height) :!class /Script/Engine.MaterialInstanceDynamic)
  (Rendering|Material|SetScalarParameterValue _returnvalue_6 "Surge Wave Height" (Variables|Default|GetSurge%20Height) :!class /Script/Engine.MaterialInstanceDynamic)
  (Rendering|Material|SetScalarParameterValue _returnvalue_6 "Tessellation Multiplier" (Variables|Default|GetTessellation%20Multiplier) :!class /Script/Engine.MaterialInstanceDynamic)
  (Rendering|Material|SetScalarParameterValue _returnvalue_6 "Tessellation Strength" (Variables|Default|GetTessellation%20Strength) :!class /Script/Engine.MaterialInstanceDynamic)
  (Rendering|Material|SetScalarParameterValue _returnvalue_6 "Foam Blur" (Variables|Default|GetFoam%20Blur) :!class /Script/Engine.MaterialInstanceDynamic)
  (Rendering|Material|SetScalarParameterValue _returnvalue_6 "Foam Height" (Variables|Default|GetFoam%20Height) :!class /Script/Engine.MaterialInstanceDynamic)
  (Rendering|Material|SetScalarParameterValue _returnvalue_6 "Foam Scale" (/ (Variables|Default|GetFoam%20Scale) _returnvalue_3) :!class /Script/Engine.MaterialInstanceDynamic)
  (Rendering|Material|SetScalarParameterValue _returnvalue_6 "Foam Speed" (* (Variables|Default|GetFoam%20Speed) 0.0025) :!class /Script/Engine.MaterialInstanceDynamic)
  (Rendering|Material|SetScalarParameterValue _returnvalue_6 "Shore Distortion Scale" (/ (Variables|Default|GetFoam%20Distortion%20Scale) _returnvalue_3) :!class /Script/Engine.MaterialInstanceDynamic)
  (Rendering|Material|SetScalarParameterValue _returnvalue_6 "Shore Distortion Speed" (* (Variables|Default|GetFoam%20Distortion%20Speed) 0.125) :!class /Script/Engine.MaterialInstanceDynamic)
  (Rendering|Material|SetScalarParameterValue _returnvalue_6 "Shore Fade" (Variables|Default|GetShore%20Fade) :!class /Script/Engine.MaterialInstanceDynamic)
  (Rendering|Material|SetScalarParameterValue _returnvalue_6 "Rain Speed" (Variables|Default|GetRaindrop%20Speed) :!class /Script/Engine.MaterialInstanceDynamic)
  (Rendering|Material|SetScalarParameterValue _returnvalue_6 "Rain Normal Power" (Variables|Default|GetRaindrop%20Normal%20Power) :!class /Script/Engine.MaterialInstanceDynamic)
  (Rendering|Material|SetScalarParameterValue _returnvalue_6 "Rain Intensity" (Variables|Default|GetRaindrop%20Intensity) :!class /Script/Engine.MaterialInstanceDynamic)
  (Rendering|Material|SetScalarParameterValue _returnvalue_6 "Rain Scale" (* _returnvalue_5 (Variables|Default|GetRaindrop%20Scale)) :!class /Script/Engine.MaterialInstanceDynamic)
  (Rendering|Material|SetTextureParameterValue _returnvalue_6 "Coral Reef Mask" (Variables|Default|GetCoral%20Reef))
  (Rendering|Material|SetScalarParameterValue _returnvalue_6 "Coral Reef Scale" (* _returnvalue_5 (Variables|Default|GetCoral%20Reef%20Scale)) :!class /Script/Engine.MaterialInstanceDynamic)
  (Rendering|Material|SetVectorParameterValue _returnvalue_6 "Color Coral Reef" (Math|Conversions|ToLinearColor(Color) (Variables|Default|GetCoral%20Reef%20Color)) :!class /Script/Engine.MaterialInstanceDynamic)
  (Rendering|Material|SetScalarParameterValue _returnvalue_6 "Coral Reef Contrast" (Variables|Default|GetCoral%20Reef%20Contrast) :!class /Script/Engine.MaterialInstanceDynamic)
  (Rendering|Material|SetScalarParameterValue _returnvalue_6 "Sea Foam Scale" (* _returnvalue_5 (Variables|Default|GetSea%20Foam%20Scale)) :!class /Script/Engine.MaterialInstanceDynamic)
  (Rendering|Material|SetScalarParameterValue _returnvalue_6 "Sea Foam Contrast" (Variables|Default|GetSea%20Foam%20Contrast) :!class /Script/Engine.MaterialInstanceDynamic)
  (Rendering|Material|SetScalarParameterValue _returnvalue_6 "Sea Foam Intensity" (Variables|Default|GetSea%20Foam%20Intensity) :!class /Script/Engine.MaterialInstanceDynamic))